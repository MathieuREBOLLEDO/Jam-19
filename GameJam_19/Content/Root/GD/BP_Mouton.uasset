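; BP_Mouton is a sheep actor that picks a random mesh and, after a start delay, runs parent logic and randomizes its speed.
; The construction script creates a dynamic material with emissive power zeroed and a red emissive color.
; TimerGroom sphere-traces for nearby pawns, re-arming its timer for BP_Loup wolves, otherwise clearing it and setting CanYouDoubleMe.
; DeathDepassement calls DestroyActor, followed by stop, hide and delayed replay logic.
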(event `self.ReceiveBeginPlay`
  (bind _arraymouton (`self.ArrayMouton`))
  (`StaticMeshComponent.SetStaticMesh` (`self.Cube`) (`|GetArrayItem` _arraymouton (`KismetMathLibrary.RandomIntegerInRange` 0 (- (`KismetArrayLibrary.Array_Length` _arraymouton) 1))))
  (`KismetSystemLibrary.Delay` (`self.DelayStart`))
  (`parent.ReceiveBeginPlay`)
  (set `self.Speed` (`KismetMathLibrary.RandomFloatInRange` (`self.SpeedMin`) (`self.SpeedMax`))))

(event `TimerGroom`
  (bind _returnvalue (`self.K2_GetActorLocation`))
  (bind _outhits (`KismetSystemLibrary.SphereTraceMultiForObjects` :`Start` _returnvalue :`End` _returnvalue :`Radius` 300.0 :`ObjectTypes` (`|MakeArray` "ObjectTypeQuery3" :!type "EObjectTypeQuery Enum") :`DrawDebugType` "ForDuration"))
  (for _array_element _outhits
    (cast `/Game/Root/GD/BP_Loup` (`.HitActor` (`GameplayStatics.BreakHitResult` _array_element))
      (:`then`
        (bind _returnvalue_2 (`KismetSystemLibrary.K2_SetTimerDelegate` (delegate `TimerGroom`) 0.1 true)))
      (:`CastFailed`
        (`KismetSystemLibrary.K2_ClearAndInvalidateTimerHandle` _returnvalue_2)
        (set `self.CanYouDoubleMe?` true)))))

(event `GetDouble`)

(event `DeathDepassement`
  (`self.K2_DestroyActor`)
  (`self.StopMoving`)
  (`SceneComponent.SetVisibility` (`self.Cube`) false false)
  (`KismetSystemLibrary.Delay` 3.0)
  (`self.Replay`)
  (`SceneComponent.SetVisibility` (`self.Cube`) true false)
  (set `self.NB_Life` 2.0))

(fn `UserConstructionScript`
  (bind _arraymouton (`self.ArrayMouton`))
  (bind _cube (`self.Cube`))
  (`parent.UserConstructionScript`)
  (`StaticMeshComponent.SetStaticMesh` (`self.Cube`) (`|GetArrayItem` _arraymouton (`KismetMathLibrary.RandomIntegerInRange` 0 (- (`KismetArrayLibrary.Array_Length` _arraymouton) 1))))
  (bind _returnvalue (`PrimitiveComponent.CreateDynamicMaterialInstance` _cube 0 (`PrimitiveComponent.GetMaterial` _cube 0) "None"))
  (set `self.DynamicMaterial` _returnvalue)
  (`MaterialInstanceDynamic.SetScalarParameterValue` _returnvalue "Emissivepower" 0.0)
  (`MaterialInstanceDynamic.SetVectorParameterValue` _returnvalue "Emissiv" (struct :`R` 1.0 :`B` 0.079394 :`A` 1.0)))