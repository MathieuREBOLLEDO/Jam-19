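; BP_Loup is the wolf in a racing game, resolving overtakes with sheep (BP_Mouton).
; Its box overlap uses one-shot flags on the sheep: a stunned sheep loses a life and dies at zero, while an unstunned one gains a life.
; A sheep reaching the life threshold shows the game-over widget.
; Restart calls the parent, then has the top-down controller check the wolf's turn.
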(event `self.ReceiveBeginPlay`
  (`parent.ReceiveBeginPlay`))

(event `self.Box.OnComponentBeginOverlap`
  (params (OverlappedComponent :type "PrimitiveComponent Object Reference") (OtherActor :type "Actor Object Reference") (OtherComp :type "PrimitiveComponent Object Reference") (OtherBodyIndex :type Integer) (bFromSweep :type Boolean) (SweepResult :type "HitResult Structure (by ref)"))
  (bind _asbp_racer (cast `/Game/Root/GD/BP_Racer` OtherActor))
  (bind _nb_life (`/Game/Root/GD/BP_Racer.NB_Life` _asbp_racer))
  (`KismetSystemLibrary.PrintString` (`KismetStringLibrary.Conv_DoubleToString` _nb_life) true true (struct :`R` 1.0 :`B` 0.061304 :`A` 1.0) 10.0)
  (bind _asbp_mouton (cast `/Game/Root/GD/BP_Mouton` _asbp_racer))
  (if (`/Game/Root/GD/BP_Racer.Stun?` _asbp_racer)
    (if (`/Game/Root/GD/BP_Racer.CanYouDoubleMe?` _asbp_mouton)
      (set `/Game/Root/GD/BP_Racer.CanYouDoubleMe?` false _asbp_mouton)
      (`/Engine/EditorBlueprintResources/StandardMacros.DecrementFloat` _nb_life
        (:`  `
          (if (<= _nb_life 0.0)
            (bind _asbp_mouton_2 (cast `/Game/Root/GD/BP_Mouton` _asbp_racer))
            (`/Game/Root/GD/BP_Mouton.DeathDepassement` _asbp_mouton_2)))))
    (elif (`/Game/Root/GD/BP_Racer.CanIDoubleYou?` _asbp_mouton)
      (set `/Game/Root/GD/BP_Racer.CanIDoubleYou?` false _asbp_mouton)
      (`self.JustedDoubled` _asbp_racer)
      (`/Engine/EditorBlueprintResources/StandardMacros.IncrementFloat` _nb_life
        (:`  `
          (if (>= _nb_life 4.0)
            (`KismetSystemLibrary.PrintString` "You lose Groomer")
            (`/Engine/EditorBlueprintResources/StandardMacros.DoOnce` false
              (:`Completed`
                (bind _returnvalue (`|CreateWidget` "/Game/Root/GD/UI/W_GameOver.W_GameOver_C"))
                (`UserWidget.AddToViewport` _returnvalue 0)
                (`WidgetBlueprintLibrary.SetInputMode_UIOnlyEx` (`GameplayStatics.GetPlayerController` 0) _returnvalue)))))))))

(event `self.Restart`
  (`parent.Restart`)
  (bind _asbp_top_down_controller (cast `/Game/TopDown/Blueprints/BP_TopDownController` (`GameplayStatics.GetPlayerController` 0)))
  (`/Game/TopDown/Blueprints/BP_TopDownController.CheckTurnLoup` _asbp_top_down_controller))

(fn `UserConstructionScript`
  (`parent.UserConstructionScript`))