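; Obstacle actor, apparently a scarecrow, with a one-in-eight chance of using an enlarged "Gabi" mesh variant.
; Timers keep its widget facing the BP_Cam camera and randomly trigger a one-off spinning dance.
; Onhit swaps the mesh for BP_EpouvantailChaos, with camera shake, explosion sound and the widget shown unless Loup is true.
; A timeline then drives camera zoom and global slow motion before resetting the camera and destroying the actor.
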(event `Dance?`
  (if (`KismetMathLibrary.RandomBool`)
    (`KismetSystemLibrary.K2_ClearAndInvalidateTimerHandle` (stale `self.ReceiveBeginPlay` _returnvalue_3))
    (bind (_direction _newtrack_0) (`Timeline|Rotation` :!via `PlayFromStart`)
      (:`Update`
        (`SceneComponent.K2_SetWorldRotation` (`self.StaticMesh`) (`KismetMathLibrary.MakeRotator` 0.0 0.0 (`KismetMathLibrary.Lerp` 0.0 720.0 _newtrack_0)) false false)))))

(event `self.ReceiveBeginPlay`
  (bind _staticmesh (`self.StaticMesh`))
  (if (== (`KismetMathLibrary.RandomIntegerInRange` 1 8) 8)
    (bind _returnvalue (`StaticMeshComponent.SetStaticMesh` _staticmesh "/Game/Environment/Props/Props/Gabi.Gabi"))
    (set `self.Gabi?` _returnvalue)
    (set `self.Chaos` "/Game/Chaos/Gabi_GeometryCollection.Gabi_GeometryCollection")
    (`SceneComponent.SetWorldScale3D` _staticmesh (6.0 6.0 6.0))
    (else
      (set `self.Chaos` "/Game/Chaos/Truc_LP_GeometryCollection.Truc_LP_GeometryCollection")
      (set `self.w_point` null)))
  (bind _returnvalue_2 (`GameplayStatics.GetActorOfClass` "/Game/Camera/BP_Cam.BP_Cam_C"))
  (set `self.CamerAmanager` _returnvalue_2)
  (`SceneComponent.SetVisibility` (`self.Widget`) false false)
  (`KismetSystemLibrary.K2_SetTimerDelegate` (delegate `CustomEvent_0`) 0.01 true)
  (set `self.NewVar_1` (`self.GetActorRelativeScale3D`))
  (bind _returnvalue_3 (`KismetSystemLibrary.K2_SetTimerDelegate` (delegate `Dance?`) (`KismetMathLibrary.RandomFloatInRange` 0.5 4.0) true)))

(event `CustomEvent_0`
  (`SceneComponent.K2_SetWorldRotation` (`self.Widget`) (`KismetMathLibrary.FindLookAtRotation` (`SceneComponent.K2_GetComponentLocation` (`self.Widget`)) (`SceneComponent.K2_GetComponentLocation` (`/Game/Camera/BP_Cam.Camer_Abase_0` (`self.CamerAmanager`)))) false false))

(event `Onhit`
  (params (`Loup*` :type Boolean))
  (bind (_returnvalue_location _returnvalue_rotation) (`KismetMathLibrary.BreakTransform` (`SceneComponent.K2_GetComponentToWorld` (`self.StaticMesh`))))
  (`PrimitiveComponent.SetCollisionEnabled` (`self.StaticMesh`) "NoCollision")
  (`|SpawnActorFromClass` "/Game/Chaos/BP_EpouvantailChaos.BP_EpouvantailChaos_C" (`KismetMathLibrary.MakeTransform` _returnvalue_location _returnvalue_rotation) "Undefined" "OverrideRootScale" null "/Game/Characters/Truc_T/Material__70.Material__70" (`self.Gabi?`) null)
  (`/Game/Camera/BP_Cam.ED_CamerAshake_Event` (`self.CamerAmanager`) 1 self)
  (`GameplayStatics.PlaySoundAtLocation` "/Game/SFX/Cues/SE_OJ_KIRAIRA_EXPLODE_Cue.SE_OJ_KIRAIRA_EXPLODE_Cue" (`PlayerCameraManager.GetCameraLocation` (`GameplayStatics.GetPlayerCameraManager` 0)) (struct) 1.0 (`GameplayStatics.GetGlobalTimeDilation`) 0.0 null null null null)
  (`SceneComponent.SetVisibility` (`self.Widget`) (not `Loup*`) false)
  (`self.K2_DetachFromActor` "KeepWorld" "KeepWorld" "KeepWorld")
  (`SceneComponent.SetHiddenInGame` (`self.StaticMesh`) true false)
  (bind (_direction _slomo _camerazoom) (`Timeline|Slomo` :!via `PlayFromStart`)
    (:`Update`
      (`/Game/Camera/BP_Cam.CameraZoom` (`self.CamerAmanager`) self _camerazoom)
      (`GameplayStatics.SetGlobalTimeDilation` _slomo))
    (:`Finished`
      (`/Game/Camera/BP_Cam.ResetOnce` (`self.CamerAmanager`))
      (`self.K2_DestroyActor`))))

(event `self.ReceiveDestroyed`)

(event `SetScore`
  (params (Score :type Integer))
  (set `self.Score` Score))

(fn `UserConstructionScript`)