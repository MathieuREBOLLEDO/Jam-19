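; BP_Obstacles is an obstacle actor that plays a slow-motion explosion reaction when its Onhit event fires, then destroys itself.
; On hit it disables and hides the mesh, triggers a BP_Cam shake, plays an explosion sound and reveals a widget.
; The Slomo timeline drives global time dilation before destruction.
; A fast looping timer billboards the widget toward the BP_Cam camera; the spawn-scale timeline is left unconnected.
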(event `self.ReceiveBeginPlay`
  (bind _returnvalue (`GameplayStatics.GetActorOfClass` "/Game/Camera/BP_Cam.BP_Cam_C"))
  (set `self.CamerAmanager` _returnvalue)
  (`SceneComponent.SetVisibility` (`self.Widget`) false false)
  (`KismetSystemLibrary.K2_SetTimerDelegate` (delegate `CustomEvent_0`) 0.01 true)
  (set `self.NewVar_1` (`self.GetActorRelativeScale3D`)))

(event `CustomEvent_0`
  (`SceneComponent.K2_SetWorldRotation` (`self.Widget`) (`KismetMathLibrary.FindLookAtRotation` (`SceneComponent.K2_GetComponentLocation` (`self.Widget`)) (`SceneComponent.K2_GetComponentLocation` (`/Game/Camera/BP_Cam.Camer_Abase_0` (`self.CamerAmanager`)))) false false))

(event `Onhit`
  (`PrimitiveComponent.SetCollisionEnabled` (`self.StaticMesh`) "NoCollision")
  (`/Game/Camera/BP_Cam.ED_CamerAshake_Event` (`self.CamerAmanager`) 1 self)
  (`GameplayStatics.PlaySoundAtLocation` "/Game/SFX/Cues/SE_OJ_KIRAIRA_EXPLODE_Cue.SE_OJ_KIRAIRA_EXPLODE_Cue" (`PlayerCameraManager.GetCameraLocation` (`GameplayStatics.GetPlayerCameraManager` 0)) (struct) 1.0 (`GameplayStatics.GetGlobalTimeDilation`) 0.0 null null null null)
  (`SceneComponent.SetVisibility` (`self.Widget`) true false)
  (`SceneComponent.SetHiddenInGame` (`self.StaticMesh`) true false)
  (bind (_direction _newtrack_0 _newtrack_1) (`Timeline|Slomo` :!via `PlayFromStart`)
    (:`Update`
      (`GameplayStatics.SetGlobalTimeDilation` _newtrack_1))
    (:`Finished`
      (`self.K2_DestroyActor`))))

(event `self.ReceiveDestroyed`)

(fn `UserConstructionScript`)