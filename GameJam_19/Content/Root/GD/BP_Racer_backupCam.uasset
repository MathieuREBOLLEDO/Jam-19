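; BP_Racer_backupCam is a racer actor that runs laps along a referenced spline, offset sideways by XOffset.
; A looping-by-restart timeline drives position and tangent-aligned rotation, with its play rate derived from spline length and Speed.
; Obstacle hits notify the obstacle and BP_Cam, score by the IsLoup flag, then pause movement for a stun followed by temporary invincibility.
; Interact queues a timed effect, currently a temporary speed boost.
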(event `StopMoving`
  (bind _spline (`self.Spline`))
  (bind _spline_2 (`self.Spline`))
  (bind (_direction _alpha) (`Timeline|Timeline_0` :!via `Stop` :!label _label)
    (:`Update`
      (bind _returnvalue (`KismetMathLibrary.Lerp` 0.0 (`SplineComponent.GetDistanceAlongSplineAtSplinePoint` _spline_2 (- (`SplineComponent.GetNumberOfSplinePoints` _spline_2) 1)) _alpha))
      (`self.K2_SetActorLocation` (`SplineComponent.GetLocationAtDistanceAlongSpline` _spline _returnvalue "World") true)
      (`self.K2_SetActorRotation` (`KismetMathLibrary.Conv_VectorToRotator` (`SplineComponent.GetTangentAtDistanceAlongSpline` _spline _returnvalue "World")) true)
      (`self.K2_SetActorLocation` (+ (* (`self.GetActorRightVector`) (`self.x_offset`)) (`self.K2_GetActorLocation`)) true))
    (:`Finished`
      (`self.Restart`)
      (bind _result (`/Engine/EditorBlueprintResources/StandardMacros.IncrementInt` (`self.NB_Turn`))
        (:`  `
          (`KismetSystemLibrary.PrintString` (`KismetStringLibrary.Conv_IntToString` _result) true false (`self.Text Color Turn`)))))))

(event `self.ReceiveBeginPlay`
  (bind _spline (`self.Spline`))
  (set `self.InitSpeed` (`self.Speed`))
  (`|ExecutionSequence`
    (:`then_0`
      (bind _returnvalue (`GameplayStatics.GetActorOfClass` "/Game/Root/GD/BP_ScoreSystem.BP_ScoreSystem_C"))
      (set `self.ScoreSystem` _returnvalue)
      (bind _returnvalue_2 (`GameplayStatics.GetActorOfClass` "/Game/Camera/BP_Cam.BP_Cam_C"))
      (set `self.NewVar_0` _returnvalue_2))
    (:`then_1`
      (set `self.Spline` (`/Game/Root/GD/BP_Spline.Spline` (`self.actor`)))
      (`TimelineComponent.SetPlayRate` (`self.Timeline_0`) (/ 1.0 (/ (`SplineComponent.GetDistanceAlongSplineAtSplinePoint` _spline (- (`SplineComponent.GetNumberOfSplinePoints` _spline) 1)) (* (`self.Speed`) 100.0))))
      (bind _returnvalue_3 (`PrimitiveComponent.CreateDynamicMaterialInstance` (`self.Cube`) 0 "/Game/LevelPrototyping/Materials/M_PrototypeGrid.M_PrototypeGrid" "None"))
      (`MaterialInstanceDynamic.SetVectorParameterValue` _returnvalue_3 "SurfaceColor" (`self.Color`))
      (goto _label :!via `PlayFromStart`))))

(event `Replay`
  (goto _label))

(event `Restart`
  (goto _label :!via `PlayFromStart`))

(event `self.ReceiveTick`
  (params (DeltaSeconds :type "Float (single-precision)"))
  (bind _spline (`/Game/Root/GD/BP_Spline.Spline` (`self.actor`)))
  (if true
    (`TimelineComponent.SetPlayRate` (`self.Timeline_0`) (/ 1.0 (/ (`SplineComponent.GetDistanceAlongSplineAtSplinePoint` _spline (- (`SplineComponent.GetNumberOfSplinePoints` _spline) 1)) (* (`self.Speed`) 10.0))))))

(event `self.Cube.OnComponentBeginOverlap`
  (params (OverlappedComponent :type "PrimitiveComponent Object Reference") (OtherActor :type "Actor Object Reference") (OtherComp :type "PrimitiveComponent Object Reference") (OtherBodyIndex :type Integer) (bFromSweep :type Boolean) (SweepResult :type "HitResult Structure (by ref)"))
  ;[1 1 1] TouchObstacles
  (bind _asbp_obstacles (cast `/Game/Root/GD/Obstalces/BP_Obstacles` OtherActor))
  (if (`self.Invincible?`)
    _
    (elif (not (`self.Stun?`))
      (`KismetSystemLibrary.PrintString` "FX_DestroyObstacle")
      (`/Game/Root/GD/Obstalces/BP_Obstacles.Onhit` _asbp_obstacles)
      (`/Game/Camera/BP_Cam.Call Desttroy` (`self.NewVar_0`))
      (`self.StopMoving`)
      (set `self.Stun?` false)
      (if (`self.IsLoup`)
        (`/Game/Root/GD/BP_ScoreSystem.Score_Event` (`self.ScoreSystem`) 0)
        (else
          (`/Game/Root/GD/BP_ScoreSystem.Score_Event` (`self.ScoreSystem`) 100)))
      (`KismetSystemLibrary.Delay` (`self.StunTime`))
      (`self.Replay`)
      (set `self.Stun?` false)
      (set `self.Invincible?` true)
      (`KismetSystemLibrary.PrintString` "FX_Blink")
      (`KismetSystemLibrary.Delay` (`self.InvincibilityDuration`))
      (set `self.Invincible?` false))))

(event `/Game/Root/GD/BPI_Interface.Interact`
  (params (Effect :type "/Game/Root/GD/MysteryBoxEffect Enum" :default "NewEnumerator0"))
  ;[1 1 1] PlayEffect
  (if (not (`self.GotEffect?`))
    (set `self.ActiveEffect` Effect)
    (set `self.GotEffect?` true)
    (`KismetSystemLibrary.K2_SetTimerDelegate` (delegate `PlayEffect`) (`self.EffectTime`))))

(event `PlayEffect`
  ;[1 1 1] PlayEffect
  (switch `/Game/Root/GD/MysteryBoxEffect` (`self.ActiveEffect`)
    (:`NewEnumerator0`
      (set `self.Speed` (* (`self.Speed`) 1.5))
      (`KismetSystemLibrary.Delay` (`self.SpeedBoostTimer`))
      (set `self.Speed` (`self.InitSpeed`))
      (set `self.GotEffect?` false))))

(fn `UserConstructionScript`
  (set `self.Spline` (`/Game/Root/GD/BP_Spline.Spline` (`self.actor`)))
  (`self.K2_SetActorLocation` (`SplineComponent.GetLocationAtSplinePoint` (`self.Spline`) 0 "World")))