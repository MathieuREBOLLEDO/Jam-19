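; Race camera actor that also runs track spawning, with zoom, shake and audio listener override to the wolf (BP_Loup).
; BeginPlay groups BP_Spline actors into tracks and starts timers placing obstacles, mystery boxes and nukes at random spline points, mostly offset to racer lanes.
; Obstacles retry blocked spots via sphere trace with a capped loop.
; A debug-style key switches tracks, and SpawnEnnemies waits for the wolf's track-position window before spawning sheep.
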(event `self.ReceiveBeginPlay`
  (bind _tracks_track1 (break `/Game/Root/GD/AllTracks` (`self.Tracks`)))
  (bind _camer_abase_0 (`self.Camer_Abase_0`))
  (bind _springarm (`self.SpringArm`))
  (bind (_track1 _track2 _track3) (break `/Game/Root/GD/AllTracks` (`self.Tracks`)))
  (`|ExecutionSequence`
    (:`then_0`
      (set `self.FoV_Base` (`CameraComponent.FieldOfView` _camer_abase_0))
      (set `self.PostProcess_Base` (`CameraComponent.PostProcessSettings` _camer_abase_0))
      (set `self.SA_Socket Offset_Base` (`SpringArmComponent.SocketOffset` _springarm))
      (set `self.SA_Target Offset_Base` (`SpringArmComponent.TargetOffset` _springarm))
      (set `self.SA_Target Arm Length_Base` (`SpringArmComponent.TargetArmLength` _springarm))
      (bind _asbp_camer_azoom (cast `/Game/Camera/BP_CamerAzoom` (`self.Camer Azoom`)))
      (set `self.Cam2_SpringArm` (`/Game/Camera/BP_CamerAzoom.SpringArm` _asbp_camer_azoom))
      (set `self.Cam2_Cam` (`/Game/Camera/BP_CamerAzoom.Camera` _asbp_camer_azoom)))
    (:`then_1`
      (set `self.Camer Azoom` (`ActorComponent.GetOwner` (`self.BP_CamerAzoom`)))
      (bind _outactors (`GameplayStatics.GetAllActorsOfClass` "/Game/Root/GD/BP_Spline.BP_Spline_C"))
      (for _array_element _outactors
        (switch `/Game/Root/GD/TracksName` (`/Game/Root/GD/BP_Spline.TracksName` _array_element)
          (:`NewEnumerator0`
            (`KismetArrayLibrary.Array_AddUnique` _track1 _array_element))
          (:`NewEnumerator1`
            (`KismetArrayLibrary.Array_AddUnique` _track2 _array_element))
          (:`NewEnumerator2`
            (`KismetArrayLibrary.Array_AddUnique` _track3 _array_element))))
      (set `self.ActualTrack` 0)
      ;[1 1 1] SapwnObstalces
      (set `self.AllSpine` _tracks_track1)
      (set `self.TimeRandom` (`KismetMathLibrary.RandomFloatInRange` (`self.TimerSpawnerMin`) (`self.TimerSpawnerMax`)))
      (`KismetSystemLibrary.K2_SetTimerDelegate` (delegate `SpawnObstacles`) (`self.TimeRandom`) true)
      (`KismetSystemLibrary.K2_SetTimer` null "SpawnMysteryBox" (`self.TimeRandom`) true)
      (`KismetSystemLibrary.K2_SetTimer` null "SpawnNuke" 15.0 true)
      (bind _returnvalue (`GameplayStatics.GetActorOfClass` "/Game/Root/GD/BP_Loup.BP_Loup_C"))
      (set `self.LoupVar` _returnvalue)
      (`PlayerController.SetAudioListenerOverride` :`self` (`GameplayStatics.GetPlayerController` 0) :`AttachToComponent` (`/Game/Root/GD/BP_Racer.Cube` _returnvalue)))
    (:`then_2`
      (bind _outactors_2 (`GameplayStatics.GetAllActorsWithTag` "FollowCam"))
      (for _array_element_2 _outactors_2
        (`self.K2_AttachToActor` _array_element_2 self "None" "KeepWorld" "KeepWorld" "KeepWorld" true)))))

(event `SpawnObstacles`
  (bind _allspine (`self.AllSpine`))
  (bind _splineoffset (`self.SplineOffset`))
  (bind _spline (`/Game/Root/GD/BP_Spline.Spline` (`|GetArrayItem` _allspine (`KismetMathLibrary.RandomIntegerInRange` 0 (- (`KismetArrayLibrary.Array_Length` _allspine) 1)))))
  (bind _returnvalue (`KismetMathLibrary.RandomFloatInRange` 0.0 (`SplineComponent.GetSplineLength` _spline)))
  ;[1 1 1] SapwnObstalces
  (set `self.SecureInfinitLoop` 0)
  (set `self.TimeRandom` (`KismetMathLibrary.RandomFloatInRange` (`self.TimerSpawnerMin`) (`self.TimerSpawnerMax`)) :!label _label)
  (bind _output_get (set `self.Spawnlocation` (`SplineComponent.GetLocationAtDistanceAlongSpline` _spline _returnvalue "World")))
  (bind _outhit (`KismetSystemLibrary.SphereTraceSingleForObjects` :`Start` _output_get :`End` _output_get :`Radius` 250.0 :`ObjectTypes` (`|MakeArray` "ObjectTypeQuery3" :!type "EObjectTypeQuery Enum") :`DrawDebugType` "ForDuration"))
  (if (`GameplayStatics.BreakHitResult` _outhit)
    (bind _result (`/Engine/EditorBlueprintResources/StandardMacros.IncrementInt` (`self.SecureInfinitLoop`))
      (:`  `
        (if (not (>= _result 10))
          (`self.CheckAgain`))))
    (else
      (set `self.SecureInfinitLoop` 0)
      (bind _returnvalue_2 (`|SpawnActorFromClass` "/Game/Root/GD/Obstalces/BP_Obstacles.BP_Obstacles_C" (`KismetMathLibrary.MakeTransform` (`self.Spawnlocation`) (`KismetMathLibrary.MakeRotFromX` (`SplineComponent.GetTangentAtDistanceAlongSpline` _spline _returnvalue "World"))) "Undefined" "OverrideRootScale" null null))
      (`KismetSystemLibrary.PrintString` "FX_SpawnObstacle")
      (`/Engine/EditorBlueprintResources/StandardMacros.IsValid` _returnvalue_2
        (:`Is Valid`
          (`self.K2_SetActorLocation` _returnvalue_2 (+ (`self.K2_GetActorLocation` _returnvalue_2) (* (`self.GetActorRightVector` _returnvalue_2) (`|GetArrayItem` _splineoffset (`KismetMathLibrary.RandomIntegerInRange` 0 (- (`KismetArrayLibrary.Array_Length` _splineoffset) 1))))) false true)
          (`self.K2_AttachToActor` _returnvalue_2 self "None" "KeepWorld" "KeepWorld" "KeepWorld" true))))))

(event `CheckAgain`
  ;[1 1 1] SapwnObstalces
  (goto _label))

(event `Key|Add`
  (params (Key :type "Key Structure"))
  (bind (_tracks_track1 _tracks_track2 _tracks_track3) (break `/Game/Root/GD/AllTracks` (`self.Tracks`)))
  (:`Pressed`
    (`/Engine/EditorBlueprintResources/StandardMacros.IncrementInt` (`self.ActualTrack`)
      (:`  `
        (if (> (`self.ActualTrack`) 1)
          (set `self.ActualTrack` 0))
        (switch `int` (`self.ActualTrack`)
          (:`0`
            (set `self.AllSpine` _tracks_track1))
          (:`1`
            (set `self.AllSpine` _tracks_track2))
          (:`2`
            (set `self.AllSpine` _tracks_track3)))
        (`self.ED_TrackChange`)))))

(event `SpawnEnnemies`
  (bind _loupvar (`self.LoupVar`))
  (bind _emplacementsurlapiste (`/Game/Root/GD/BP_Racer.EmplacementSurLapiste` _loupvar))
  (bind (_returnvalue_location _returnvalue_rotation) (`KismetMathLibrary.BreakTransform` (`SplineComponent.GetTransformAtTime` (`/Game/Root/GD/BP_Spline.Spline` (`|GetArrayItem` (`self.AllSpine`))) 0.0 "World" false false)))
  (bind _result (`/Engine/EditorBlueprintResources/StandardMacros.IncrementFloat` (`self.SpawnEnemieWaiting`))
    (:`  `
      (for _ (range (+ (`KismetMathLibrary.FTrunc` (- _result 1.0)) 1))
        (if (and (<= _emplacementsurlapiste 0.75) (>= _emplacementsurlapiste 0.4)) :!label _label_2
          (bind _returnvalue (`|SpawnActorFromClass` "/Game/Root/GD/BP_Mouton.BP_Mouton_C" (`KismetMathLibrary.MakeTransform` _returnvalue_location _returnvalue_rotation (7.0 7.0 7.0)) "Undefined" "OverrideRootScale" null null))
          (set `/Game/Root/GD/BP_Mouton.DelayStart` (/ (`self.SpawnEnemieWaiting`) 10.0) _returnvalue)
          (set `/Game/Root/GD/BP_Racer.NB_Turn` (+ (`/Game/Root/GD/BP_Racer.NB_Turn` _loupvar) 1) _returnvalue)
          (set `self.SpawnEnemieWaiting` 0.0)
          (else
            (`KismetSystemLibrary.Delay` 0.1)
            (goto _label_2)))))))

(event `Key|²`
  (params (Key :type "Key Structure"))
  (:`Pressed`
    (switch `int` (stale `Call Desttroy` _output_get) :!label _label_3
      (:`1`
        (`GameplayStatics.PlayWorldCameraShake` "/Game/Root/GD/ScreenShake/SS_Ashake_PetitFrere.SS_Ashake_PetitFrere_C" (`PlayerCameraManager.GetCameraLocation` (`GameplayStatics.GetPlayerCameraManager` 0)) 0.0 1000.0)
        (`KismetSystemLibrary.PrintString` "SHAAAAKE")))))

(event `Call Desttroy`
  (bind _output_get (set `self.Level` 1))
  (goto _label_3))

(event `ED_CamerAshake_Event` :!signature `self.ED_CamerAshake`
  (params (Level :type Integer) (Target :type "Actor Object Reference")))

(event `ResetOnce`
  ;[1 1 1] Comment
)

(event `CameraZoom`
  (params (ActorSource :type "Actor Object Reference") (CameraZoomAlpha :type "Float (double-precision)"))
  (bind _sa_target_arm_length_base (`self.SA_Target Arm Length_Base`))
  ;[1 1 1] Comment
  (set `self.Camera Zoom Alpha` CameraZoomAlpha)
  (set `SpringArmComponent.TargetArmLength` (`KismetMathLibrary.Lerp` _sa_target_arm_length_base (/ _sa_target_arm_length_base 12.0) (`self.Camera Zoom Alpha`)) (`self.SpringArm`)))

(event `ReturnCamBase`)

(fn `SpawnMysteryBox`
  (bind _allspine (`self.AllSpine`))
  (bind _splineoffset (`self.SplineOffset`))
  (bind _output (`|GetArrayItem` _allspine (`KismetMathLibrary.RandomIntegerInRange` 0 (- (`KismetArrayLibrary.Array_Length` _allspine) 1))))
  (bind _returnvalue (`KismetMathLibrary.RandomFloatInRange` 0.0 (`SplineComponent.GetSplineLength` (`/Game/Root/GD/BP_Spline.Spline` _output))))
  (set `self.TimeRandom` (`KismetMathLibrary.RandomFloatInRange` (* (`self.TimerSpawnerMin`) 1.8) (* (`self.TimerSpawnerMax`) 1.8)))
  (set `self.Spawnlocation` (`SplineComponent.GetLocationAtDistanceAlongSpline` (`/Game/Root/GD/BP_Spline.Spline` _output) _returnvalue "World"))
  (bind _returnvalue_2 (`|SpawnActorFromClass` "/Game/Root/GD/BP_MysteryBox.BP_MysteryBox_C" (`KismetMathLibrary.MakeTransform` (`self.Spawnlocation`) (`KismetMathLibrary.MakeRotFromX` (`SplineComponent.GetTangentAtDistanceAlongSpline` (`/Game/Root/GD/BP_Spline.Spline` _output) _returnvalue "World")) (0.5 0.5 0.5)) "Undefined" "OverrideRootScale" null "NewEnumerator0" null))
  (`KismetSystemLibrary.PrintString` "FX_SpawnMysteryBox")
  (`/Engine/EditorBlueprintResources/StandardMacros.IsValid` _returnvalue_2
    (:`Is Valid`
      (`self.K2_SetActorLocation` _returnvalue_2 (+ (`self.K2_GetActorLocation` _returnvalue_2) (* (`self.GetActorRightVector` _returnvalue_2) (`|GetArrayItem` _splineoffset (`KismetMathLibrary.RandomIntegerInRange` 0 (- (`KismetArrayLibrary.Array_Length` _splineoffset) 1))))) false true))))

(fn `SpawnNuke`
  (bind _allspine (`self.AllSpine`))
  (bind _output (`|GetArrayItem` _allspine (`KismetMathLibrary.RandomIntegerInRange` 0 (- (`KismetArrayLibrary.Array_Length` _allspine) 1))))
  (bind _returnvalue (`KismetMathLibrary.RandomFloatInRange` 0.0 (`SplineComponent.GetSplineLength` (`/Game/Root/GD/BP_Spline.Spline` _output))))
  (set `self.TimeRandom` (`KismetMathLibrary.RandomFloatInRange` (* (`self.TimerSpawnerMin`) 1.8) (* (`self.TimerSpawnerMax`) 1.8)))
  (set `self.Spawnlocation` (`SplineComponent.GetLocationAtDistanceAlongSpline` (`/Game/Root/GD/BP_Spline.Spline` _output) _returnvalue "World"))
  (bind _returnvalue_2 (`|SpawnActorFromClass` "/Game/Root/GD/BP_Nuke.BP_Nuke_C" (`KismetMathLibrary.MakeTransform` (`self.Spawnlocation`) (`KismetMathLibrary.MakeRotFromX` (`SplineComponent.GetTangentAtDistanceAlongSpline` (`/Game/Root/GD/BP_Spline.Spline` _output) _returnvalue "World")) (0.5 0.5 0.5)) "Undefined" "OverrideRootScale" null "NewEnumerator4" null))
  (`KismetSystemLibrary.PrintString` "FX_Nuke")
  (`/Engine/EditorBlueprintResources/StandardMacros.IsValid` _returnvalue_2
    (:`Is Valid`
      (`self.K2_SetActorLocation` _returnvalue_2 (+ (`self.K2_GetActorLocation` _returnvalue_2) (* (`self.GetActorRightVector` _returnvalue_2) 450.0)) false true)
      (`self.K2_AttachToActor` _returnvalue_2 self "None" "KeepWorld" "KeepWorld" "KeepWorld" true))))

(fn `UserConstructionScript`
  (bind _returnvalue (`PrimitiveComponent.CreateDynamicMaterialInstance` (`self.Plane`) 0 null "None"))
  (`MaterialInstanceDynamic.SetVectorParameterValue` _returnvalue "BaseColor" (`self.Value`))
  (`KismetArrayLibrary.Array_Clear` (`self.Array_Racer`))
  (`KismetArrayLibrary.Array_Clear` (`self.SplineOffset`))
  (bind _outactors (`GameplayStatics.GetAllActorsOfClass` "/Game/Root/GD/BP_Racer.BP_Racer_C"))
  (bind _output_get (set `self.Array_Racer` _outactors))
  (for _array_element _output_get
    (`KismetArrayLibrary.Array_Add` (`self.SplineOffset`) (`/Game/Root/GD/BP_Racer.x_offset` _array_element))))